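; BP_IconCreator is a capture-stage actor that displays a static mesh, skeletal mesh or spawned actor for a scene capture, apparently to create icons.
; The capture's show-only list isolates the stage and attached actor, while centering uses bounds to offset each asset.
; Setters control asset transform, animation pose, overlay material and light shadows.
; Orbit, zoom and FOV functions adjust the spring-arm camera, with the light holder mirroring its rotation.
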(fn ConstructionScript
  (Utilities|Array|AddUnique (Variables|/Script/Engine.SceneCaptureComponent|GetShowOnlyActors (Variables|Default|GetSceneCaptureComponent2D)) self))

(fn Center
  (bind _skeletalmesh (Variables|Default|GetSkeletalMesh))
  (bind _staticmesh (Variables|Default|GetStaticMesh))
  (bind _attachedactor (Variables|Default|GetAttachedActor))
  (bind (_min _max) (Components|StaticMesh|GetLocalBounds _staticmesh))
  (Transformation|SetRelativeLocation _staticmesh (/ (+ _min _max) -2.0) false false)
  (Transformation|SetRelativeLocation _skeletalmesh (- (Transformation|GetWorldLocation _skeletalmesh) (.Origin (Collision|GetComponentBounds _skeletalmesh))) false false)
  (Variables|Default|GetAttachedActor
    (:then
      (Transformation|SetActorRelativeLocation _attachedactor (- (Transformation|GetActorLocation _attachedactor) (.Origin (Collision|GetActorBounds _attachedactor false true)))))
    (:else)))

(fn ZoomCamera
  (params (Value :type Float%20%28double-precision%29))
  (bind _springarm (Variables|Default|GetSpringArm))
  (Variables|/Script/Engine.SpringArmComponent|SetTargetArmLength _springarm (+ (Variables|/Script/Engine.SpringArmComponent|GetTargetArmLength _springarm) Value)))

(fn ChangeCameraRotation
  (params (Z :type Float%20%28double-precision%29) (Y :type Float%20%28double-precision%29))
  (bind _springarm (Variables|Default|GetSpringArm))
  (bind _relativerotation (Variables|/Script/Engine.SceneComponent|GetRelativeRotation _springarm))
  (Transformation|SetRelativeRotation (Variables|Default|GetSpringArm) (Math|Rotator|MakeRotator 0.0 (Math|Float|Clamp(Float) (+ (.pitch _relativerotation) (* Y -1.0)) -89.99 89.99) (+ (.yaw _relativerotation) Z)) false false)
  (Transformation|SetRelativeRotation (Variables|Default|GetLightHolder) (Variables|/Script/Engine.SceneComponent|GetRelativeRotation (Variables|Default|GetSpringArm)) false false))

(fn SetCameraRotation
  (params (NewRotation :type Rotator))
  (Transformation|SetRelativeRotation (Variables|Default|GetSpringArm) (Math|Rotator|MakeRotator 0.0 (.pitch NewRotation) (.yaw NewRotation)) false false)
  (Transformation|SetRelativeRotation (Variables|Default|GetLightHolder) (Math|Rotator|MakeRotator 0.0 (.pitch NewRotation) (.yaw NewRotation)) false false))

(fn SetCameraLocation
  (params (NewLocation :type Vector))
  (Transformation|SetRelativeLocation (Variables|Default|GetSpringArm) NewLocation false false))

(fn SetCameraDistance
  (params (Distance :type Float%20%28single-precision%29))
  (Variables|/Script/Engine.SpringArmComponent|SetTargetArmLength (Variables|Default|GetSpringArm) Distance))

(fn SetActor
  (params (Actor :type Actor%20Class%20Reference))
  (Utilities|FlowControl|Sequence
    (:then_0
      (bind _attachedactor (Variables|Default|GetAttachedActor)
        (:then
          (Actor|DestroyActor _attachedactor))
        (:else)))
    (:then_1
      (bind _actor (LocalVariables|GetActor)
        (:then
          (bind _returnvalue (Game|SpawnActorfromClass _actor (Math|Transform|MakeTransform "0, 0, 0" "0, 0, 0" "1.000000,1.000000,1.000000") "Undefined" "MultiplyWithRoot" 0 0))
          (Variables|Default|SetAttachedActor _returnvalue)
          (bind _attachedactor_2 (Variables|Default|GetAttachedActor)
            (:then
              (Transformation|AttachComponentToComponent _attachedactor_2 (Variables|Default|GetAssetHolder) "None" "KeepRelative" "KeepRelative" "KeepRelative" true)
              (Utilities|Array|Add (Variables|/Script/Engine.SceneCaptureComponent|GetShowOnlyActors (Variables|Default|GetSceneCaptureComponent2D)) (Variables|Default|GetAttachedActor)))
            (:else)))
        (:else)))))

(fn SetStaticMesh
  (params (NewMesh :type Static%20Mesh%20Object%20Reference))
  (Components|StaticMesh|SetStaticMesh (Variables|Default|GetStaticMesh) NewMesh))

(fn SetSkeletalMesh
  (params (NewMesh :type Skeletal%20Mesh%20Object%20Reference))
  (Components|SkeletalMesh|SetSkeletalMeshAsset (Variables|Default|GetSkeletalMesh) NewMesh))

(fn SetOverlayMaterial
  (params (NewOverlayMaterial :type Material%20Interface%20Object%20Reference))
  (Rendering|Material|SetOverlayMaterial (Variables|Default|GetStaticMesh) NewOverlayMaterial :!class /Script/Engine.MeshComponent)
  (Variables|Default|GetAttachedActor
    (:then
      (Utilities|FlowControl|Sequence
        (:then_0
          (for _array_element (Actor|GetComponentsByClass (Variables|Default|GetAttachedActor) "/Script/Engine.StaticMeshComponent")
            (Rendering|Material|SetOverlayMaterial _array_element NewOverlayMaterial :!class /Script/Engine.MeshComponent)))
        (:then_1
          (for _array_element_2 (Actor|GetComponentsByClass (Variables|Default|GetAttachedActor) "/Script/Engine.SkeletalMeshComponent")
            (Rendering|Material|SetOverlayMaterial _array_element_2 NewOverlayMaterial :!class /Script/Engine.MeshComponent)))))
    (:else)))

(fn SetAnim
  (params (NewAnimToPlay :type Animation%20Asset%20Object%20Reference))
  (Components|Animation|SetAnimation (Variables|Default|GetSkeletalMesh) NewAnimToPlay))

(fn SetAnimPosition
  (params (Initial%20Position :type Float%20%28single-precision%29))
  (Components|Animation|SetPosition (Variables|Default|GetSkeletalMesh) Initial%20Position false))

(fn SetAssetScale
  (params (NewScale :type Vector))
  (Transformation|SetRelativeScale3D (Variables|Default|GetAssetHolder) NewScale))

(fn SetAssetRotation
  (params (NewRotation :type Rotator))
  (Transformation|SetRelativeRotation (Variables|Default|GetAssetHolder) NewRotation false false))

(fn SetCastShadows1
  (params (bNewValue :type Boolean))
  (Rendering|Components|Light|SetCastShadows (Variables|Default|GetLight1) bNewValue))

(fn SetCastShadows2
  (params (bNewValue :type Boolean))
  (Rendering|Components|Light|SetCastShadows (Variables|Default|GetLight2) bNewValue))

(fn SetCastShadows3
  (params (bNewValue :type Boolean))
  (Rendering|Components|Light|SetCastShadows (Variables|Default|GetLight3) bNewValue))

(fn SetFieldOfView
  (params (Field%20of%20View :type Float%20%28single-precision%29))
  (Variables|/Script/Engine.SceneCaptureComponent2D|SetFOVAngle (Variables|Default|GetSceneCaptureComponent2D) Field%20of%20View))